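; Monopoly game mode Blueprint that serves as the UI layer, creating the menus and binding their buttons to game actions defined outside these graphs.
; Starting a game passes shuffled token meshes and materials to StartGame.
; Property, house-upgrade and debt-payment screens are fresh widgets filled from MonopolyProperties, whose selected items drive selling, downgrading or upgrading.
; Escape toggles the in-game menu once play starts, and numpad keys trigger cheats.
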(event Custom|ShowSameGroups
  (bind _buyhousemenu (Variables|Default|GetBuyHouseMenu))
  (CallFunction|GenerateSameGroupTiles)
  (Class|MPGameMode|ShowSameGroupMenu)
  (EventDispatchers|BindEventtoOnClicked (Variables|/Script/Licenta.BuyHouseWidget|GetBackButton _buyhousemenu) (delegate Custom|BackToGame))
  (EventDispatchers|BindEventtoOnClicked (Variables|/Script/Licenta.BuyHouseWidget|GetBuyHouseButton _buyhousemenu) (delegate Custom|BuyHouse)))

(event Custom|End%20Turn
  (Class|MPGameMode|NextPlayer))

(event Custom|BackToPlayMenu
  (Class|MPGameMode|HidePropertiesMenu))

(event Custom|Show%20Properties
  (bind _ownedpropertiesmenu (Variables|Default|GetOwnedPropertiesMenu))
  (bind _downgradebutton (Variables|/Script/Licenta.OwnedPropertiesWidget|GetDowngradeButton _ownedpropertiesmenu))
  (bind _sellbutton (Variables|/Script/Licenta.OwnedPropertiesWidget|GetSellButton _ownedpropertiesmenu))
  (CallFunction|GenerateTiles)
  (Class|MPGameMode|ShowPropertiesMenu)
  (Utilities|FlowControl|Sequence
    (:then_0
      (Widget|SetVisibility _sellbutton "Collapsed")
      (Widget|SetVisibility _downgradebutton "Collapsed"))
    (:then_1
      (EventDispatchers|BindEventtoOnClicked (Variables|/Script/Licenta.OwnedPropertiesWidget|GetBackButton _ownedpropertiesmenu) (delegate Custom|BackToPlayMenu))
      (EventDispatchers|BindEventtoOnClicked _sellbutton (delegate Custom|SellProp))
      (EventDispatchers|BindEventtoOnClicked _downgradebutton (delegate Custom|DownGradeProperty)))))

(event Custom|SellProp
  (bind _asmonopoly_property (Utilities|Casting|CastToMonopolyProperty (Class|ListView|GetSelectedItem (Variables|/Script/Licenta.OwnedPropertiesWidget|GetProperties (Variables|Default|GetOwnedPropertiesMenu)))))
  (Class|MPGameMode|SellProperty (Variables|/Script/Licenta.MonopolyProperty|GetPropertyPosition _asmonopoly_property) 0)
  (Class|MPGameMode|HidePropertiesMenu)
  (CallFunction|ShowProperties))

(event Custom|BackToGame
  (Class|MPGameMode|HideSameGroupMenu))

(event Custom|DowngradeEvent
  (bind _asmonopoly_property (Utilities|Casting|CastToMonopolyProperty (Class|ListView|GetSelectedItem (Variables|/Script/Licenta.OwnedPropsPayRestWidget|GetProperties (Variables|Default|GetPayRestMenu)))))
  (Class|MPGameMode|SellHouse _asmonopoly_property 0)
  (Class|MPGameMode|RecalculateRestInformation))

(event Custom|SellEvent
  (bind _asmonopoly_property (Utilities|Casting|CastToMonopolyProperty (Class|ListView|GetSelectedItem (Variables|/Script/Licenta.OwnedPropsPayRestWidget|GetProperties (Variables|Default|GetPayRestMenu)))))
  (Class|MPGameMode|SellProperty (Class|MonopolyProperty|GetPropertyPosition _asmonopoly_property) 0)
  (Class|MPGameMode|RecalculateRestInformation))

(event Custom|ShowStartMenu
  (Class|MPGameMode|HandleShowStartMenu))

(event Custom|ContinueEvent
  (Class|MPGameMode|ContinuePay))

(event Custom|BuyHouse
  (bind _asmonopoly_house_property (Utilities|Casting|CastToMonopolyHouseProperty (Class|ListView|GetSelectedItem (Variables|/Script/Licenta.BuyHouseWidget|GetProperties_1 (Variables|Default|GetBuyHouseMenu)))))
  (Class|MPGameMode|UpgradeProperty _asmonopoly_house_property 0)
  (Class|MPGameMode|HideSameGroupMenu)
  (CallFunction|ShowSameGroups))

(event Custom|BackToMenu
  (Class|MPGameMode|HandleBacktoInitialMenu))

(event Custom|QuitGame
  (Game|QuitGame 0 "Quit" false))

(event Custom|RollTheDice
  (Class|MPGameMode|SetRollDiceAnimationTimer))

(event Custom|GameStart
  (Variables|Default|SetGameStarted true)
  (Widget|SetVisibility (Variables|Default|GetStartMenu) "Collapsed")
  (bind _staticmeshlist (CallFunction|GenerateStaticMeshList))
  (bind _colormaterials (CallFunction|GenerateStaticMeshColors))
  (Class|MPGameMode|StartGame (Game|GetPlayerController 0) _staticmeshlist _colormaterials))

(event Custom|BuyProp
  (Class|MPGameMode|BuyProperty 0 0))

(event Custom|DownGradeProperty
  (bind _asmonopoly_property (Utilities|Casting|CastToMonopolyProperty (Class|ListView|GetSelectedItem (Variables|/Script/Licenta.OwnedPropertiesWidget|GetProperties (Variables|Default|GetOwnedPropertiesMenu)))))
  (Class|MPGameMode|SellHouse _asmonopoly_property 0)
  (Class|MPGameMode|HidePropertiesMenu)
  (CallFunction|ShowProperties))

(event EventBeginPlay
  (bind _initialmenu (Variables|Default|GetInitialMenu))
  (bind _playmenu (Variables|Default|GetPlayMenu))
  (bind _startmenu (Variables|Default|GetStartMenu))
  (CallFunction|GenerateWidgets)
  (Class|MPGameMode|Initialize)
  (EventDispatchers|BindEventtoOnClicked (Variables|/Script/Licenta.InitialWidget|GetStart _initialmenu) (delegate Custom|ShowStartMenu))
  (EventDispatchers|BindEventtoOnClicked (Variables|/Script/Licenta.InitialWidget|GetQuit _initialmenu) (delegate Custom|QuitGame))
  (EventDispatchers|BindEventtoOnClicked (Variables|/Script/Licenta.InGameWidget|GetQuitGame (Variables|Default|GetInGameMenu)) (delegate Custom|QuitGame))
  (EventDispatchers|BindEventtoOnClicked (Variables|/Script/Licenta.PlayWidget|GetRollTheDiceButton _playmenu) (delegate Custom|RollTheDice))
  (EventDispatchers|BindEventtoOnClicked (Variables|/Script/Licenta.PlayWidget|GetBuyButton _playmenu) (delegate Custom|BuyProp))
  (EventDispatchers|BindEventtoOnClicked (Variables|/Script/Licenta.PlayWidget|GetPropertiesButton _playmenu) (delegate Custom|Show%20Properties))
  (EventDispatchers|BindEventtoOnClicked (Variables|/Script/Licenta.PlayWidget|GetUpgradeButton _playmenu) (delegate Custom|ShowSameGroups))
  (EventDispatchers|BindEventtoOnClicked (Variables|/Script/Licenta.PlayWidget|GetEndTurnButton _playmenu) (delegate Custom|End%20Turn))
  (EventDispatchers|BindEventtoOnClicked (Variables|/Script/Licenta.StartGameWidget|GetBack _startmenu) (delegate Custom|BackToMenu))
  (EventDispatchers|BindEventtoOnClicked (Variables|/Script/Licenta.StartGameWidget|GetInit _startmenu) (delegate Custom|GameStart)))

(event EventPlayDiceRollSound
  (Audio|PlaySound2D "/Game/Animations/DiceRollSoundWave.DiceRollSoundWave" 1.0 1.0 0.0 0 0))

(event EventGenerateTilesforRestWidget
  (CallFunction|GenerateTilesforRestWidgetFunction))

(event EventBindPayRestButtons
  (bind _payrestmenu (Variables|Default|GetPayRestMenu))
  (EventDispatchers|BindEventtoOnClicked (Variables|/Script/Licenta.OwnedPropsPayRestWidget|GetContinueButton _payrestmenu) (delegate Custom|ContinueEvent))
  (EventDispatchers|BindEventtoOnClicked (Variables|/Script/Licenta.OwnedPropsPayRestWidget|GetSellButton _payrestmenu) (delegate Custom|SellEvent))
  (EventDispatchers|BindEventtoOnClicked (Variables|/Script/Licenta.OwnedPropsPayRestWidget|GetDowngradeButton _payrestmenu) (delegate Custom|DowngradeEvent)))

(event Input|KeyboardEvents|Escape
  (params (Key :type Key%20Structure :default "None"))
  (bind _playmenu (Variables|Default|GetPlayMenu))
  (bind _ingamemenu (Variables|Default|GetInGameMenu))
  (:Pressed
    (if (Variables|Default|GetGameStarted)
      (if (Widget|IsVisible _ingamemenu)
        (Widget|SetVisibility _ingamemenu "Collapsed")
        (Widget|SetVisibility _playmenu "Visible")
        (else
          (Widget|SetVisibility _playmenu "Collapsed")
          (Widget|SetVisibility _ingamemenu "Visible"))))))

(event Input|KeyboardEvents|NumPadOne
  (params (Key :type Key%20Structure :default "None"))
  (:Pressed
    (Class|MPGameMode|CHEATLose)))

(event Input|KeyboardEvents|NumPadTwo
  (params (Key :type Key%20Structure :default "None"))
  (:Pressed
    (Class|MPGameMode|CHEATWin)))

(event Input|KeyboardEvents|NumPadFour
  (params (Key :type Key%20Structure :default "None"))
  (:Pressed
    (Class|MPGameMode|CHEATRest)))

(event Input|KeyboardEvents|NumPadFive
  (params (Key :type Key%20Structure :default "None"))
  (:Pressed
    (Class|MPGameMode|CHEATBuyHouse)))

(fn ConstructionScript)

(fn GenerateStaticMeshList
  (bind _mesharray (LocalVariables|GetMeshArray))
  (Utilities|Array|Add _mesharray "/Game/Shapes/cup.cup")
  (Utilities|Array|Add _mesharray "/Game/Shapes/Dog.Dog")
  (Utilities|Array|Add _mesharray "/Game/Shapes/hat.hat")
  (Utilities|Array|Add _mesharray "/Game/Shapes/shoes.shoes")
  (Utilities|Array|Shuffle _mesharray)
  (return _mesharray))

(fn GenerateWidgets
  (bind _returnvalue (Game|GetPlayerController 0))
  (bind _returnvalue_2 (UserInterface|CreateWidget "/Game/Widgets/Initial.Initial_C"))
  (bind _output_get (Variables|Default|SetInitialMenu _returnvalue_2))
  (UserInterface|Viewport|AddtoViewport _output_get 0)
  (bind _returnvalue_3 (UserInterface|CreateWidget "/Game/Widgets/Play.Play_C"))
  (bind _output_get_2 (Variables|Default|SetPlayMenu _returnvalue_3))
  (UserInterface|Viewport|AddtoViewport _output_get_2 0)
  (Widget|SetVisibility _output_get_2 "Collapsed")
  (Variables|/Script/Licenta.PlayWidget|SetDiceRollMediaPlayer _output_get_2 "/Game/Animations/DiceRollMedia.DiceRollMedia")
  (Variables|/Script/Licenta.PlayWidget|SetDiceRollSource _output_get_2 "/Game/Animations/DiceRollWithSound3S.DiceRollWithSound3S")
  (bind _returnvalue_4 (UserInterface|CreateWidget "/Game/Widgets/StartGame.StartGame_C"))
  (bind _output_get_3 (Variables|Default|SetStartMenu _returnvalue_4))
  (UserInterface|Viewport|AddtoViewport _output_get_3 0)
  (Widget|SetVisibility _output_get_3 "Collapsed")
  (bind _returnvalue_5 (UserInterface|CreateWidget "/Game/Widgets/InGameMenu.InGameMenu_C"))
  (bind _output_get_4 (Variables|Default|SetInGameMenu _returnvalue_5))
  (UserInterface|Viewport|AddtoViewport _output_get_4 0)
  (Widget|SetVisibility _output_get_4 "Collapsed")
  (bind _returnvalue_6 (UserInterface|CreateWidget "/Game/Widgets/GameOver.GameOver_C"))
  (bind _output_get_5 (Variables|Default|SetGameOverMenu _returnvalue_6))
  (UserInterface|Viewport|AddtoViewport _output_get_5 0)
  (Widget|SetVisibility _output_get_5 "Collapsed")
  (bind _returnvalue_7 (UserInterface|CreateWidget "/Game/Widgets/OwnedProperties.OwnedProperties_C"))
  (bind _output_get_6 (Variables|Default|SetOwnedPropertiesMenu _returnvalue_7))
  (UserInterface|Viewport|AddtoViewport _output_get_6 0)
  (Widget|SetVisibility _output_get_6 "Collapsed")
  (bind _returnvalue_8 (UserInterface|CreateWidget "/Game/Widgets/OwnedPropertiesToPayRestBP.OwnedPropertiesToPayRestBP_C"))
  (bind _output_get_7 (Variables|Default|SetPayRestMenu _returnvalue_8))
  (UserInterface|Viewport|AddtoViewport _output_get_7 0)
  (Widget|SetVisibility _output_get_7 "Collapsed")
  (bind _returnvalue_9 (UserInterface|CreateWidget "/Game/Widgets/SameGroupForUpgrade.SameGroupForUpgrade_C"))
  (bind _output_get_8 (Variables|Default|SetBuyHouseMenu _returnvalue_9))
  (UserInterface|Viewport|AddtoViewport _output_get_8 0)
  (Widget|SetVisibility _output_get_8 "Collapsed")
  (Variables|/Script/Engine.PlayerController|SetbShowMouseCursor _returnvalue true)
  (Input|EnableInput _returnvalue)
  (Input|SetInputModeGameandUI _returnvalue (Variables|Default|GetInitialMenu) "DoNotLock" false)
  (Input|SetInputModeGameandUI _returnvalue (Variables|Default|GetPlayMenu) "DoNotLock" false)
  (Input|SetInputModeGameandUI _returnvalue (Variables|Default|GetStartMenu) "DoNotLock" false)
  (Input|SetInputModeGameandUI _returnvalue (Variables|Default|GetInGameMenu) "DoNotLock" false))

(fn GenerateStaticMeshColors
  (bind _colors (LocalVariables|GetColors))
  (Utilities|Array|Add _colors "/Game/CustomMeshes/ChestsColor.ChestsColor")
  (Utilities|Array|Add _colors "/Game/CustomMeshes/ChancesColor.ChancesColor")
  (Utilities|Array|Add _colors "/Game/CustomMeshes/BrownProp.BrownProp")
  (Utilities|Array|Add _colors "/Game/CustomMeshes/BlueProp.BlueProp")
  (Utilities|Array|Shuffle _colors)
  (return _colors))

(fn GenerateTiles
  (bind _returnvalue (UserInterface|CreateWidget "/Game/Widgets/OwnedProperties.OwnedProperties_C"))
  (bind _output_get (Variables|Default|SetOwnedPropertiesMenu _returnvalue))
  (UserInterface|Viewport|AddtoViewport _output_get 0)
  (Widget|SetVisibility _output_get "Visible")
  (bind _asowned_properties (Utilities|Casting|CastToOwnedProperties _output_get))
  (bind _returnvalue_2 (Class|MPGameMode|GetParticipant))
  (Default|SetCurrentPlayer _asowned_properties _returnvalue_2)
  (for _array_element (Variables|Default|GetMonopolyProperties)
    (if (Class|MonopolyProperty|IsOwnable _array_element)
      (Class|ListView|AddItem (Variables|/Script/Licenta.OwnedPropertiesWidget|GetProperties _asowned_properties) _array_element))))

(fn GenerateSameGroupTiles
  (Utilities|FlowControl|Sequence
    (:then_0
      (bind _returnvalue (UserInterface|CreateWidget "/Game/Widgets/SameGroupForUpgrade.SameGroupForUpgrade_C"))
      (bind _output_get (Variables|Default|SetBuyHouseMenu _returnvalue))
      (UserInterface|Viewport|AddtoViewport _output_get 0)
      (Widget|SetVisibility _output_get "Visible")
      (bind _assame_group_for_upgrade (Utilities|Casting|CastToSameGroupForUpgrade _output_get))
      (bind _returnvalue_2 (Class|MPGameMode|GetParticipant))
      (Variables|/Game/Widgets/SameGroupForUpgrade.SameGroupForUpgrade_C|SetCurrentPlayer _returnvalue _returnvalue_2))
    (:then_1
      (for _array_element (Variables|Default|GetMonopolyProperties)
        (bind _asmonopoly_house_property (Utilities|Casting|CastToMonopolyHouseProperty _array_element))
        (bind _returnvalue_3 (Class|MPGameMode|GetParticipant))
        (bind _returnvalue_4 (Class|MPGameMode|GetProperty (Class|ParticipantPawn|GetPlayerPosition _returnvalue_3)))
        (bind _asmonopoly_house_property_2 (Utilities|Casting|CastToMonopolyHouseProperty _returnvalue_4))
        (if (and (Class|MonopolyProperty|IsOwnable _asmonopoly_house_property) (Utilities|Enum|Equal(Enum) (Class|MonopolyHouseProperty|GetPropGroup _asmonopoly_house_property) (Class|MonopolyHouseProperty|GetPropGroup _asmonopoly_house_property_2)))
          (Class|ListView|AddItem (Variables|/Script/Licenta.BuyHouseWidget|GetProperties_1 _assame_group_for_upgrade) _array_element))))))

(fn GenerateTilesforRestWidgetFunction
  (bind _returnvalue (UserInterface|CreateWidget "/Game/Widgets/OwnedPropertiesToPayRestBP.OwnedPropertiesToPayRestBP_C"))
  (bind _output_get (Variables|Default|SetPayRestMenu _returnvalue))
  (UserInterface|Viewport|AddtoViewport _output_get 0)
  (Widget|SetVisibility _output_get "Visible")
  (bind _returnvalue_2 (Class|MPGameMode|GetParticipant))
  (bind _output_get_2 (Variables|/Script/Licenta.OwnedPropsPayRestWidget|SetCurrentPlayer _output_get _returnvalue_2))
  (for _array_element (Variables|Default|GetMonopolyProperties)
    (if (== (Class|MonopolyProperty|GetPropertyOwner _array_element) _output_get_2)
      (Class|ListView|AddItem (Variables|/Script/Licenta.OwnedPropsPayRestWidget|GetProperties _output_get) _array_element))))